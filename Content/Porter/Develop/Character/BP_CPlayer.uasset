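; BP_CPlayer is the player character Blueprint that manages item pickups and the resulting player and hero stats.
; BeginPlay seeds stats from a struct and creates the stats, item-choice, bonus-item and hero widgets.
; Items from DT_Item add stat deltas, update stacked inventory counts, then branch by type into random grants, stack-count bonuses or debuff-to-buff replacement.
; Tab opens a time-freezing item choice, R toggles the hero screen, and other keys are debug hooks.
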(event Custom|ItemGetdown
  ;[1 1 1] Comment
  (Widget|RemovefromParent (Variables|Default|GetWB_Choose%20Item_main_1))
  (Variables|/Script/Engine.PlayerController|SetbShowMouseCursor (Game|GetPlayerController 0) false)
  (Input|SetInputModeGameOnly (Game|GetPlayerController 0) true)
  (Utilities|Time|SetGlobalTimeDilation 1.0))

(event Custom|GetItem+4/+5
  ;[0.02353 0.1373 0.01569] Comment
  (for _index (range 1 (Math|Random|RandomIntegerinRange 4 5))
    _))

(event Custom|GetItem+2/+3
  ;[0.02353 0.1373 0.01569] 랜덤 아이템 획득 2~3
  (for _index (range 1 (Math|Random|RandomIntegerinRange 2 3))
    _))

(event Custom|Item_
  (params (RowName :type Name))
  ;[1 1 1] Comment
  (bind _returnvalue (Utilities|GetDataTableRow "/Game/Porter/Develop/Item/Table/DT_Item.DT_Item" RowName)
    (:then
      (bind (_type _typevalue) (Utilities|ItemStats _returnvalue)
        (:then_10
          (Utilities|FlowControl|Sequence
            (:then_0
              (CallFunction|AddItem RowName)
              (CallFunction|Update))
            (:then_1
              (switch Utilities|FlowControl|Switch|SwitchonEnum_ItemType _type
                (:NewEnumerator3
                  (Utilities|RandomItem _typevalue))
                (:NewEnumerator4
                  (|AllStatsItem _returnvalue _typevalue RowName))
                (:NewEnumerator6
                  (|RemoveDebuff))))))))))

(event EventBeginPlay
  ;[1 1 1] BeginPlay
  (Utilities|FlowControl|Sequence
    (:then_0
      (CallFunction|BeginPlayerStats (Variables|Default|GetST_PlayerStats))
      (bind _returnvalue (UserInterface|CreateWidget "/Game/Porter/Develop/Item/WB/WB_Text.WB_Text_C" (Game|GetPlayerController 0)))
      (bind _output_get (Variables|Default|SetWB_Stats _returnvalue))
      (UserInterface|Viewport|AddtoViewport _output_get 0)
      (bind _returnvalue_2 (UserInterface|CreateWidget "/Game/Porter/Develop/Item/WB/WB_ChooseItem_main.WB_ChooseItem_main_C" (Game|GetPlayerController 0)))
      (bind _output_get_2 (Variables|Default|SetWB_Choose%20Item_main _returnvalue_2))
      (Default|BeginPlay _output_get_2)
      (bind _returnvalue_3 (UserInterface|CreateWidget "/Game/Porter/Develop/Item/Drag/WB_Hero_Main.WB_Hero_Main_C" (Game|GetPlayerController 0))) ; 용병 드래그
      (Variables|Default|SetWB_Hero%20Int _returnvalue_3)
      (bind _returnvalue_4 (UserInterface|CreateWidget "/Game/Porter/Develop/Item/WB/WB_GetAddItem_main.WB_GetAddItem_main_C" (Game|GetPlayerController 0))) ; 추가 아이템
      (bind _output_get_3 (Variables|Default|SetWB_GetAddItem_main _returnvalue_4))
      (Default|BeginPlay _output_get_3)
      (bind _returnvalue_5 (UserInterface|CreateWidget "/Game/Porter/Develop/Item/WB/WB_ChooseItem_main1.WB_ChooseItem_main1_C" (Game|GetPlayerController 0)))
      (bind _output_get_4 (Variables|Default|SetWB_Choose%20Item_main_1 _returnvalue_5))
      (Default|BeginPlay _output_get_4))))

(event Collision|EventActorBeginOverlap
  (params (OtherActor :type Actor%20Object%20Reference)))

(event EventTick
  (params (DeltaSeconds :type Float%20%28single-precision%29)))

(event Input|KeyboardEvents|Tab
  (params (Key :type Key%20Structure :default "None"))
  (bind _returnvalue (Game|GetPlayerController 0))
  ;[1 1 1] Comment
  (:Pressed
    (Default|TNumber3 (Variables|Default|GetWB_Choose%20Item_main_1))
    (UserInterface|Viewport|AddtoViewport (Variables|Default|GetWB_Choose%20Item_main_1) 0)
    (Variables|/Script/Engine.PlayerController|SetbShowMouseCursor _returnvalue true)
    (Input|SetInputModeUIOnly _returnvalue (Variables|Default|GetWB_Choose%20Item_main) "DoNotLock" true)
    (Utilities|Time|SetGlobalTimeDilation 0.0)))

(event Input|KeyboardEvents|U
  (params (Key :type Key%20Structure :default "None"))
  (:Pressed
    (CallFunction|Item "FinestAmulet")))

(event Input|KeyboardEvents|6
  (params (Key :type Key%20Structure :default "None"))
  ;[0.02353 0.1373 0.01569] Comment
  (:Pressed
    (for _array_element (Variables|/Game/Porter/Develop/Item/Drag/WB_Hero_Main.WB_Hero_Main_C|GetHero%20Index%20Array (Variables|Default|GetWB_Hero%20Int))
      (Development|PrintString (Utilities|String|ToString(Integer) _array_element)))))

(event Input|KeyboardEvents|R
  (params (Key :type Key%20Structure :default "None"))
  ;[1 1 1] Comment
  (:Pressed
    (Utilities|FlowControl|FlipFlop
      (:A
        (UserInterface|Viewport|AddtoViewport (Variables|Default|GetWB_Hero%20Int) 0)
        (Variables|/Script/Engine.PlayerController|SetbShowMouseCursor (Game|GetPlayerController 0) true)
        (Input|SetInputModeGameandUI (Game|GetPlayerController 0) (Variables|Default|GetWB_Hero%20Int) "LockOnCapture" true true))
      (:B
        (Widget|RemovefromParent (Variables|Default|GetWB_Hero%20Int))
        (Variables|/Script/Engine.PlayerController|SetbShowMouseCursor (Game|GetPlayerController 0) false)
        (Input|SetInputModeGameOnly (Game|GetPlayerController 0) true)))))

(fn ConstructionScript)

(fn BeginPlayerStats
  (params (ST_PlayerStats :type ST%20Player%20Stats%20Structure%20%28by%20ref%29))
  (bind (_playerwalkspeed _playermaxstamina _playerstamina _playerrunspeed _playerheronumber _playermaxhp _playerhp _heroattackspeed _heromeleedamage _herocasterdamage _herocriticalchance _herocriticaldamage) (Utilities|Struct|BreakST_PlayerStats ST_PlayerStats))
  (bind (_playerwalkspeed_2 _playermaxstamina_2 _playerstamina_2 _playerrunspeed_2 _playerheronumber_2 _playermaxhp_2 _playerhp_2 _heroattackspeed_2 _heromeleedamage_2 _herocasterdamage_2 _herocriticalchance_2 _herocriticaldamage_2) (Utilities|Struct|BreakST_PlayerStats ST_PlayerStats))
  (Variables|Default|SetPlayer%20WalkSpeed _playerwalkspeed)
  (Variables|Default|SetPlayer%20MaxStamina _playermaxstamina)
  (Variables|Default|SetPlayer%20Stamina _playerstamina)
  (Variables|Default|SetPlayer%20RunSpeed _playerrunspeed)
  (Variables|Default|SetPlayer%20HeroNumber _playerheronumber)
  (Variables|Default|SetPlayer%20MaxHP _playermaxhp)
  (Variables|Default|SetPlayer%20HP _playerhp)
  (Variables|Default|SetHero%20AttackSpeed _heroattackspeed)
  (Variables|Default|SetHero%20MeleeDamage _heromeleedamage)
  (Variables|Default|SetHero%20CasterDamage _herocasterdamage)
  (Variables|Default|SetHero%20CriticalChance _herocriticalchance)
  (Variables|Default|SetHero%20CriticalDamage _herocriticaldamage)
  (Class|PPlayer|UpdateStats (Utilities|Struct|MakePlayerStatsStruct _playerwalkspeed_2 _playerrunspeed_2 _playermaxstamina_2 33.0 2e+01 1e+01 _playerheronumber_2 _playermaxhp_2 _heroattackspeed_2 _heromeleedamage_2 _herocasterdamage_2 _herocriticalchance_2 _herocriticaldamage_2)))

(fn AddItem
  (params (RowName :type Name%20%28by%20ref%29))
  (bind _player_getitemlist (Variables|Default|GetPlayer%20GetItemList))
  (bind _player_getitemlist_2 (Variables|Default|GetPlayer%20GetItemList))
  (bind (_name _count) (Utilities|Struct|BreakST_GetItem _player_getitemlist))
  (bind (_name_2 _count_2) (Utilities|Struct|BreakST_GetItem _player_getitemlist_2))
  (bind _returnvalue (Utilities|Array|FindItem _name RowName))
  (if (Utilities|Array|ContainsItem (.Name (Utilities|Struct|BreakST_GetItem (Variables|Default|GetPlayer%20GetItemList))) RowName)
    (Utilities|Array|SetArrayElem _count _returnvalue (+ (Utilities|Array|Get(acopy) _count _returnvalue) 1))
    (Default|ItemUpdate (Variables|Default|GetWB_Stats))
    (else
      (Utilities|Array|Add _name_2 RowName)
      (Utilities|Array|Add _count_2 1)
      (Default|ItemUpdate (Variables|Default|GetWB_Stats)))))

(fn Update
  (if (>= (Variables|Default|GetPlayer%20HeroNumber) 0) ; 용병 수가 음수가 되지 않게
    (Class|PPlayer|UpdateStats (Utilities|Struct|MakePlayerStatsStruct (Variables|Default|GetPlayer%20WalkSpeed) (Variables|Default|GetPlayer%20RunSpeed) (Variables|Default|GetPlayer%20MaxStamina) 33.0 2e+01 1e+01 (Variables|Default|GetPlayer%20HeroNumber) (- (Variables|Default|GetPlayer%20MaxHP) 5) (Variables|Default|GetHero%20AttackSpeed) (Variables|Default|GetHero%20MeleeDamage) (Variables|Default|GetHero%20CasterDamage) (Variables|Default|GetHero%20CriticalChance) (Variables|Default|GetHero%20CriticalDamage)))
    (else
      (Class|PPlayer|UpdateStats (Utilities|Struct|MakePlayerStatsStruct (Variables|Default|GetPlayer%20WalkSpeed) (Variables|Default|GetPlayer%20RunSpeed) (Variables|Default|GetPlayer%20MaxStamina) 33.0 2e+01 1e+01 0 (- (Variables|Default|GetPlayer%20MaxHP) 5) (Variables|Default|GetHero%20AttackSpeed) (Variables|Default|GetHero%20MeleeDamage) (Variables|Default|GetHero%20CasterDamage) (Variables|Default|GetHero%20CriticalChance) (Variables|Default|GetHero%20CriticalDamage))))))

(fn AllstatsT+3/F-3
  (params (Condition :type Boolean))
  (if Condition
    (Variables|Default|SetPlayer%20WalkSpeed (+ (Variables|Default|GetPlayer%20WalkSpeed) 1.2e+02))
    (Variables|Default|SetPlayer%20MaxStamina (+ (Variables|Default|GetPlayer%20MaxStamina) 3e+01))
    (Variables|Default|SetPlayer%20RunSpeed (+ (Variables|Default|GetPlayer%20RunSpeed) 1.2e+02))
    (Variables|Default|SetPlayer%20HeroNumber (+ (Variables|Default|GetPlayer%20HeroNumber) 3))
    (Variables|Default|SetPlayer%20MaxHP (+ (Variables|Default|GetPlayer%20MaxHP) 3))
    (Variables|Default|SetHero%20AttackSpeed (+ (Variables|Default|GetHero%20AttackSpeed) 3e+01))
    (Variables|Default|SetHero%20MeleeDamage (+ (Variables|Default|GetHero%20MeleeDamage) 3e+01))
    (Variables|Default|SetHero%20CasterDamage (+ (Variables|Default|GetHero%20CasterDamage) 3e+01))
    (Variables|Default|SetHero%20CriticalChance (+ (Variables|Default|GetHero%20CriticalChance) 15.0))
    (Variables|Default|SetHero%20CriticalDamage (+ (Variables|Default|GetHero%20CriticalDamage) 3e+01))
    (else
      (Variables|Default|SetPlayer%20WalkSpeed (+ (Variables|Default|GetPlayer%20WalkSpeed) -1.2e+02))
      (Variables|Default|SetPlayer%20MaxStamina (+ (Variables|Default|GetPlayer%20MaxStamina) -3e+01))
      (Variables|Default|SetPlayer%20RunSpeed (+ (Variables|Default|GetPlayer%20RunSpeed) -1.2e+02))
      (Variables|Default|SetPlayer%20HeroNumber (+ (Variables|Default|GetPlayer%20HeroNumber) -3))
      (Variables|Default|SetPlayer%20MaxHP (+ (Variables|Default|GetPlayer%20MaxHP) -3))
      (Variables|Default|SetHero%20AttackSpeed (+ (Variables|Default|GetHero%20AttackSpeed) -3e+01))
      (Variables|Default|SetHero%20MeleeDamage (+ (Variables|Default|GetHero%20MeleeDamage) -3e+01))
      (Variables|Default|SetHero%20CasterDamage (+ (Variables|Default|GetHero%20CasterDamage) -3e+01))
      (Variables|Default|SetHero%20CriticalChance (+ (Variables|Default|GetHero%20CriticalChance) -15.0))
      (Variables|Default|SetHero%20CriticalDamage (+ (Variables|Default|GetHero%20CriticalDamage) -3e+01)))))

(fn NewFunction
  (params (B :type Enum_ItemType%20Enum :default "NewEnumerator0") (LastIndex :type Integer))
  (bind _outrownames (DataTable|GetDataTableRowNames "/Game/Porter/Develop/Item/Table/DT_Item.DT_Item"))
  (for _array_element _outrownames
    (bind _returnvalue (Utilities|GetDataTableRow "/Game/Porter/Develop/Item/Table/DT_Item.DT_Item" _array_element)
      (:then
        (if (Utilities|Enum|Equal(Enum) (.Type (Utilities|Struct|BreakST_Item _returnvalue)) B)
          (Utilities|Array|Add (Variables|Default|GetChooseItemList3) _array_element)))))
  (for _index (range 1 LastIndex)
    (bind _output_get (Variables|Default|SetSaveName (.OutItem (Utilities|Array|Random (Variables|Default|GetChooseItemList3)))))
    (Default|GetAddItem (Variables|Default|GetWB_GetAddItem_main) _output_get))
  (Utilities|Array|Clear (Variables|Default|GetChooseItemList3)))

(fn WBMainVi
  (Variables|/Script/Engine.PlayerController|SetbShowMouseCursor (Game|GetPlayerController 0) true)
  (Input|SetInputModeUIOnly (Game|GetPlayerController 0) (Variables|Default|GetWB_GetAddItem_main) "DoNotLock" false)
  (UserInterface|Viewport|AddtoViewport (Variables|Default|GetWB_GetAddItem_main) 0))

(fn DebuffReplacement
  (params (ItemToFind :type Name%20%28by%20ref%29) (RowName :type Name))
  (bind _player_getitemlist (Variables|Default|GetPlayer%20GetItemList))
  (bind (_name _count) (Utilities|Struct|BreakST_GetItem _player_getitemlist))
  (bind _returnvalue (Utilities|Array|FindItem _name ItemToFind))
  (bind _returnvalue_2 (Utilities|GetDataTableRow "/Game/Porter/Develop/Item/Table/DT_Item.DT_Item" ItemToFind)
    (:then
      (if (!= _returnvalue -1)
        (for _index (range 1 (Utilities|Array|Get(acopy) _count _returnvalue))
          (bind _returnvalue_3 (Utilities|GetDataTableRow "/Game/Porter/Develop/Item/Table/DT_Item.DT_Item" RowName)
            (:then
              (Utilities|ItemStats _returnvalue_3))))
        (CallFunction|Update)
        (Utilities|Array|RemoveIndex _name _returnvalue)
        (Utilities|Array|RemoveIndex _count _returnvalue)
        (Default|ItemUpdate (Variables|Default|GetWB_Stats))))))

(fn AddItem0
  (params (ST_Item :type ST%20Item%20Structure%20%28by%20ref%29))
  (bind _name (Utilities|Struct|BreakST_Item ST_Item))
  (bind _player_getitemlist (Variables|Default|GetPlayer%20GetItemList))
  (bind _player_getitemlist_2 (Variables|Default|GetPlayer%20GetItemList))
  (bind (_name_2 _count) (Utilities|Struct|BreakST_GetItem _player_getitemlist))
  (bind (_name_3 _count_2) (Utilities|Struct|BreakST_GetItem _player_getitemlist_2))
  (bind _returnvalue (Utilities|Array|FindItem _name_2 _name))
  (if (Utilities|Array|ContainsItem (.Name (Utilities|Struct|BreakST_GetItem (Variables|Default|GetPlayer%20GetItemList))) _name)
    (Utilities|Array|SetArrayElem _count _returnvalue (+ (Utilities|Array|Get(acopy) _count _returnvalue) 1))
    (Default|ItemUpdate (Variables|Default|GetWB_Stats))
    (else
      (Utilities|Array|Add _name_3 _name)
      (Utilities|Array|Add _count_2 1)
      (Default|ItemUpdate (Variables|Default|GetWB_Stats)))))