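; BP_Player is the player character for a test map, handling movement, jump, pause and game-over screens.
; BeginPlay adds the Enhanced Input mapping context and the player HUD widget.
; Move input follows control yaw, while the game-over and pause actions swap the HUD for UI-only menus with a cursor.
; The unpause branch restores game input but never clears IsTestPause or re-adds the HUD.
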(event Input|EnhancedActionEvents|EnhancedInputActionIA_TestMapPlayerMove
  (params (ActionValue :type Vector%202D%20Structure) (ElapsedSeconds :type Float%20%28double-precision%29) (TriggeredSeconds :type Float%20%28double-precision%29) (InputAction :type Input%20Action%20Object%20Reference :default "/Game/Porter/Develop/Widgets/Level_TestMap/TestMapPlayer/TestMapPlayerInput/IA_TestMapPlayerMove.IA_TestMapPlayerMove"))
  (bind _returnvalue (Pawn|GetControlRotation :!class /Script/Engine.Pawn))
  (bind _returnvalue_2 (Pawn|GetControlRotation :!class /Script/Engine.Pawn))
  (Pawn|Input|AddMovementInput (Math|Vector|GetRightVector (Math|Rotator|MakeRotator (.roll _returnvalue) 0.0 (.yaw _returnvalue))) (.y ActionValue) false)
  (Pawn|Input|AddMovementInput (Math|Vector|GetForwardVector (Math|Rotator|MakeRotator (.roll _returnvalue_2) 0.0 (.yaw _returnvalue_2))) (.x ActionValue) false))

(event Input|EnhancedActionEvents|EnhancedInputActionIA_TestMapPlayerJump
  (params (ActionValue :type Boolean) (ElapsedSeconds :type Float%20%28double-precision%29) (TriggeredSeconds :type Float%20%28double-precision%29) (InputAction :type Input%20Action%20Object%20Reference :default "/Game/Porter/Develop/Widgets/Level_TestMap/TestMapPlayer/TestMapPlayerInput/IA_TestMapPlayerJump.IA_TestMapPlayerJump"))
  (:Started
    (Character|Jump)))

(event Input|EnhancedActionEvents|EnhancedInputActionIA_TestMapGameOver
  (params (ActionValue :type Boolean) (ElapsedSeconds :type Float%20%28double-precision%29) (TriggeredSeconds :type Float%20%28double-precision%29) (InputAction :type Input%20Action%20Object%20Reference :default "/Game/Porter/Develop/Widgets/Level_TestMap/TestMapPlayer/TestMapPlayerInput/IA_TestMapGameOver.IA_TestMapGameOver"))
  (bind _returnvalue (Game|GetPlayerController 0))
  (:Started
    (Input|DisableInput 0)
    (Widget|RemovefromParent (Variables|Default|GetAsTestMapPlayer))
    (bind _returnvalue_2 (UserInterface|CreateWidget "/Game/Porter/Develop/Widgets/Level_TestMap/TestMapWidget/WBP_GameOver.WBP_GameOver_C"))
    (bind _output_get (Variables|Default|SetAsTestGameOver _returnvalue_2))
    (UserInterface|Viewport|AddtoViewport _output_get 0)
    (Variables|/Script/Engine.PlayerController|SetbShowMouseCursor _returnvalue true)
    (Input|SetInputModeUIOnly _returnvalue _returnvalue_2 "DoNotLock" false)))

(event Input|EnhancedActionEvents|EnhancedInputActionIA_TestMapPause
  (params (ActionValue :type Boolean) (ElapsedSeconds :type Float%20%28double-precision%29) (TriggeredSeconds :type Float%20%28double-precision%29) (InputAction :type Input%20Action%20Object%20Reference :default "/Game/Porter/Develop/Widgets/Level_TestMap/TestMapPlayer/TestMapPlayerInput/IA_TestMapPause.IA_TestMapPause"))
  (bind _returnvalue (Game|GetPlayerController 0))
  (:Started
    (Widget|RemovefromParent (Variables|Default|GetAsTestMapPlayer))
    (if (not (Variables|Default|GetbIsTestPause))
      (Variables|Default|SetbIsTestPause true)
      (bind _returnvalue_2 (UserInterface|CreateWidget "/Game/Porter/Develop/Widgets/Level_TestMap/TestMapWidget/WBP_Pause.WBP_Pause_C"))
      (bind _output_get (Variables|Default|SetAsPause _returnvalue_2))
      (UserInterface|Viewport|AddtoViewport _output_get 0)
      (Input|SetInputModeUIOnly _returnvalue _returnvalue_2 "DoNotLock" false)
      (Variables|/Script/Engine.PlayerController|SetbShowMouseCursor _returnvalue true)
      (Game|SetGamePaused true)
      (else
        (Widget|RemovefromParent (Variables|Default|GetAsPause))
        (Game|SetGamePaused false)
        (Input|SetInputModeGameOnly _returnvalue false)
        (Variables|/Script/Engine.PlayerController|SetbShowMouseCursor _returnvalue false)))))

(event EventBeginPlay
  (Input|AddMappingContext (PlayerController|LocalPlayerSubsystems|GetEnhancedInputLocalPlayerSubsystem (Game|GetPlayerController 0)) "/Game/Porter/Develop/Widgets/Level_TestMap/TestMapPlayer/TestMapPlayerInput/IMC_TestMapPlayer.IMC_TestMapPlayer" 0 "(bIgnoreAllPressedKeysUntilRelease=True,bForceImmediately=False,bNotifyUserSettings=False)")
  (bind _returnvalue (UserInterface|CreateWidget "/Game/Porter/Develop/Widgets/Level_TestMap/TestMapWidget/WBP_TestMapPlayer.WBP_TestMapPlayer_C"))
  (bind _output_get (Variables|Default|SetAsTestMapPlayer _returnvalue))
  (UserInterface|Viewport|AddtoViewport _output_get 0))

(event Collision|EventActorBeginOverlap
  (params (OtherActor :type Actor%20Object%20Reference)))

(event EventTick
  (params (DeltaSeconds :type Float%20%28single-precision%29)))

(fn ConstructionScript)